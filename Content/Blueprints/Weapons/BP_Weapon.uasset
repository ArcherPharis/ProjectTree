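; BP_Weapon is a weapon actor that supplies hit feedback and knockback through two custom events.
; LaunchTarget shakes the first player's camera on every call, then launches characters tagged Launchable along the weapon owner's forward vector with upward lift.
; HitFXWeapon spawns a hit particle at the struck actor's location.
; Hit detection is absent here, so both events depend on being called with a target.
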(event `self.LaunchTarget`
  (params (characterToLaunch :type "Character Object Reference"))
  (bind (_returnvalue_x _returnvalue_y) (`KismetMathLibrary.BreakVector` (* (`self.GetActorForwardVector` (`self.GetOwner`)) 150.0)))
  (`PlayerController.ClientStartCameraShake` :`self` (`GameplayStatics.GetPlayerController` 0) :`Shake` "/Game/Blueprints/Player/GAS/Melee/BP_Hit_CameraShake.BP_Hit_CameraShake_C" :`Scale` 3.0)
  (if (`self.ActorHasTag` characterToLaunch "Launchable")
    (`Character.LaunchCharacter` characterToLaunch (`KismetMathLibrary.MakeVector` _returnvalue_x _returnvalue_y 200.0) false false)))

(event `self.HitFXWeapon`
  (params (actorHit :type "Actor Object Reference"))
  (`GameplayStatics.SpawnEmitterAtLocation` "/Game/FXVarietyPack/Particles/P_ky_hit2.P_ky_hit2" (`self.K2_GetActorLocation` actorHit)))

(fn `UserConstructionScript`)