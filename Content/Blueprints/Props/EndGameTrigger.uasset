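; EndGameTrigger is a level-end volume that triggers the win sequence when an actor tagged Player overlaps its box.
; It plays the player character's winning montage and switches input to UI-only.
; After a short delay, it has the player controller show the endgame screen, pauses the game, shows the mouse cursor and plays ending music.
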(event `self.Box.OnComponentBeginOverlap`
  (params (OverlappedComponent :type "PrimitiveComponent Object Reference") (OtherActor :type "Actor Object Reference") (OtherComp :type "PrimitiveComponent Object Reference") (OtherBodyIndex :type Integer) (bFromSweep :type Boolean) (SweepResult :type "HitResult Structure (by ref)"))
  (if (`self.ActorHasTag` OtherActor "Player")
    (bind _asplayer_character_controller (cast `PlayerCharacterController` (`GameplayStatics.GetPlayerController` 0)))
    (bind _asplayer_character (cast `PlayerCharacter` (`Controller.K2_GetPawn` _asplayer_character_controller)))
    (`PlayerCharacter.PlayWinningMontage` _asplayer_character)
    (`WidgetBlueprintLibrary.SetInputMode_UIOnlyEx` _asplayer_character_controller null)
    (`KismetSystemLibrary.Delay` 2.0)
    (`PlayerCharacterController.SwitchToEndgameScreen` _asplayer_character_controller)
    (`GameplayStatics.SetGamePaused` true)
    (set `PlayerController.bShowMouseCursor` true _asplayer_character_controller)
    (`GameplayStatics.PlaySound2D` "/Game/Audio/LTJENDINGMusic.LTJENDINGMusic" 1.0 1.0 0.0 null null)))

(fn `UserConstructionScript`)