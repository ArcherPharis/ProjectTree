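; BP_Worm is a worm enemy Blueprint that can knock a character away.
; Its LaunchTarget event launches the given character along the worm's forward vector by a supplied force plus a fixed upward boost, then shakes the first player's camera.
; A timeline-driven rise from the start location by WormRiseAmount is present but disconnected, so it never runs.
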(event `self.ReceiveBeginPlay`)

(event `self.LaunchTarget`
  (params (force :type "Float (single-precision)") (targetToLaunch :type "Character Object Reference"))
  (bind (_returnvalue_x _returnvalue_y) (`KismetMathLibrary.BreakVector` (* (`self.GetActorForwardVector`) force)))
  (`self.LaunchCharacter` targetToLaunch (`KismetMathLibrary.MakeVector` _returnvalue_x _returnvalue_y 700.0) false false)
  (`PlayerController.ClientStartCameraShake` :`self` (`GameplayStatics.GetPlayerController` 0) :`Shake` "/Game/Blueprints/Player/GAS/Melee/BP_Hit_CameraShake.BP_Hit_CameraShake_C" :`Scale` 4.0))

(fn `UserConstructionScript`)